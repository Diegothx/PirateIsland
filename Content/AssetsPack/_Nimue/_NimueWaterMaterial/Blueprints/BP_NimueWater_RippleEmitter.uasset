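; BP_NimueWater_RippleEmitter is an actor that emits water ripples beneath the player for the Nimue water material.
; On BeginPlay it activates the NSWaterRipple component and caches the first BP_ThirdPersonCharacter found in the level.
; Each Tick it follows that character's X and Y while keeping its own height.
; The author's note marks it as an example, with the component meant to live on the character to avoid Tick cost.
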(event `self.ReceiveBeginPlay`
  ;[1 0 0] Move this component to your character blueprint, do not use this as it is! (bad for performance due to Event Tick)
  (`ActorComponent.Activate` (`self.NS_WaterRipple`) false)
  (bind _outactors (`GameplayStatics.GetAllActorsOfClass` "/Game/Blueprints/ThirdPersonPirate/BP_ThirdPersonCharacter.BP_ThirdPersonCharacter_C"))
  (bind _output (`|GetArrayItem` _outactors))
  (`/Engine/EditorBlueprintResources/StandardMacros.IsValid` _output
    (:`Is Valid`
      (set `self.PlayerCharacterRef` _output))))

(event `self.ReceiveTick`
  (params (DeltaSeconds :type "Float (single-precision)"))
  (bind (_returnvalue_x _returnvalue_y _returnvalue_z) (`KismetMathLibrary.BreakVector` (`self.K2_GetActorLocation`)))
  ;[1 0 0] Move this component to your character blueprint, do not use this as it is! (bad for performance due to Event Tick)
  (`self.K2_SetActorLocation` (`KismetMathLibrary.MakeVector` (.x (`SceneComponent.K2_GetComponentLocation` (`Actor.RootComponent` (`self.PlayerCharacterRef`)))) (.y (`SceneComponent.K2_GetComponentLocation` (`Actor.RootComponent` (`self.PlayerCharacterRef`)))) _returnvalue_z)))

(fn `UserConstructionScript`)