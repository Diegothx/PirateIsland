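; BP_NimueWater_Body builds a tiled water surface from static mesh planes with a simple distance-based LOD.
; The construction script lays a grid around the central WaterPlane, attaching collision-free tiles spaced by PlaneSpacing.
; Tiles inside HighResRadius use the LOD0 branch and material, the rest LOD1.
; Construction and BeginPlay both write HighResRadius to MPC_NimueWater to size the material's world position offset mask.
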(event `self.ReceiveBeginPlay`
  (`KismetMaterialLibrary.SetScalarParameterValue` "/Game/AssetsPack/_Nimue/_NimueWaterMaterial/Materials/MaterialParameterCollections/MPC_NimueWater.MPC_NimueWater" "HighResRadius" (`self.HighResRadius`)) ; passes the high res radius to a material parameter collection to determine the size of the WPO mask
)

(fn `UserConstructionScript`
  (bind _waterplane (`self.WaterPlane`))
  (bind _planespacing (`self.PlaneSpacing`))
  ;[1 1 1] This is a simple LOD system for the water plane meshes. Set GridSizeX and GridSizeY to control the total size and HighResRadius to determine how many/far high res planes are spawned
  (`KismetMaterialLibrary.SetScalarParameterValue` "/Game/AssetsPack/_Nimue/_NimueWaterMaterial/Materials/MaterialParameterCollections/MPC_NimueWater.MPC_NimueWater" "HighResRadius" (`self.HighResRadius`)) ; passes the high res radius to a material parameter collection to determine the size of the WPO mask
  (for _index (range (/ (`self.GridSizeX`) -1) (+ (/ (`self.GridSizeX`) 1) 1))
    (for _index_2 (range (/ (`self.GridSizeY`) -1) (+ (/ (`self.GridSizeY`) 1) 1))
      (if (not (and (== _index_2 0) (== _index 0)))
        (bind _returnvalue (`KismetMathLibrary.MakeVector` (* _index _planespacing) (* _planespacing _index_2)))
        (bind _output_get (set `self.InRadius` (< (`KismetMathLibrary.VSize` _returnvalue) (`self.HighResRadius`))))
        (if _output_get
          (bind _returnvalue_2 (`KismetMathLibrary.Conv_VectorToTransform` _returnvalue))
          (bind _returnvalue_3 (`AddComponent|NODE_AddStaticMeshComponent-8` :`RelativeTransform` _returnvalue_2))
          (`SceneComponent.K2_AttachToComponent` _returnvalue_3 _waterplane "None" "KeepRelative" "KeepRelative" "KeepRelative" true)
          (`PrimitiveComponent.SetCollisionEnabled` _returnvalue_3 "NoCollision")
          (`PrimitiveComponent.SetMaterial` _returnvalue_3 0 "/Game/AssetsPack/_Nimue/_NimueWaterMaterial/Materials/MI_NimueWater_LOD0.MI_NimueWater_LOD0")
          (else
            (bind _returnvalue_4 (`AddComponent|NODE_AddStaticMeshComponent-0` :`RelativeTransform` _returnvalue_2))
            (`SceneComponent.K2_AttachToComponent` _returnvalue_4 _waterplane "None" "KeepRelative" "KeepRelative" "KeepRelative" true)
            (`PrimitiveComponent.SetCollisionEnabled` _returnvalue_4 "NoCollision")
            (`PrimitiveComponent.SetMaterial` _returnvalue_4 0 "/Game/AssetsPack/_Nimue/_NimueWaterMaterial/Materials/MI_NimueWater_LOD1.MI_NimueWater_LOD1")))))))