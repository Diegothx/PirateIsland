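; BP_NimueWater_RippleCapturer drives an orthographic scene capture that supplies ripple capture data for the Nimue water material.
; Each Tick it looks up the first BP_NimueWater_RippleEmitter and moves the capture to that actor's X and Y, keeping its own height.
; It publishes the capture position and ortho width to MPC_NimueWater.
; A graph note marks this per-Tick setup as costly, intending the component for the character Blueprint.
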(event `self.ReceiveTick`
  (params (DeltaSeconds :type "Float (single-precision)"))
  (bind _scenecapturecomponent2d (`self.SceneCaptureComponent2D`))
  (bind _returnvalue (`SceneComponent.K2_GetComponentLocation` _scenecapturecomponent2d))
  ;[1 0 0] Move this component to your character blueprint, do not use this as it is! (bad for performance due to Event Tick)
  (bind _outactors (`GameplayStatics.GetAllActorsOfClass` "/Game/AssetsPack/_Nimue/_NimueWaterMaterial/Blueprints/BP_NimueWater_RippleEmitter.BP_NimueWater_RippleEmitter_C"))
  (bind _output_get (set `self.WaterRippleDrawerRef` (`|GetArrayItem` _outactors)))
  (`SceneComponent.K2_SetWorldLocation` (`self.SceneCaptureComponent2D`) (`KismetMathLibrary.MakeVector` (.x (`self.K2_GetActorLocation` _output_get)) (.y (`self.K2_GetActorLocation` _output_get)) (.z _returnvalue)) false false)
  (`KismetMaterialLibrary.SetVectorParameterValue` "/Game/AssetsPack/_Nimue/_NimueWaterMaterial/Materials/MaterialParameterCollections/MPC_NimueWater.MPC_NimueWater" "CapturePosition" (`KismetMathLibrary.Conv_VectorToLinearColor` _returnvalue))
  (`KismetMaterialLibrary.SetScalarParameterValue` "/Game/AssetsPack/_Nimue/_NimueWaterMaterial/Materials/MaterialParameterCollections/MPC_NimueWater.MPC_NimueWater" "CaptureSize" (`SceneCaptureComponent2D.OrthoWidth` _scenecapturecomponent2d)))

(fn `UserConstructionScript`)