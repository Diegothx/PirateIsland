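; BP_Chest is a chest that opens when the third-person player character enters its Reachable area and closes when they leave.
; Overlap events play the open or close animation on the chest mesh, guarded by an IsChestOpen flag.
; Tick bobs the front and back E-key tooltips with a sine wave.
; EvalShowTooltip_Event shows those tooltips only while the root has more than four child components.
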(event `self.ReceiveBeginPlay`)

(event `self.ReceiveTick`
  (params (DeltaSeconds :type "Float (single-precision)"))
  (bind _returnvalue (* (`KismetMathLibrary.Sin` (* (`KismetSystemLibrary.GetGameTimeInSeconds`) 3.0)) 0.75))
  ; Move Ekey Tooltip up and down
  (`SceneComponent.K2_AddLocalOffset` (`self.FrontEkey`) (`KismetMathLibrary.MakeVector` 0.0 _returnvalue) false false)
  (`SceneComponent.K2_AddLocalOffset` (`self.BackEKey`) (`KismetMathLibrary.MakeVector` 0.0 _returnvalue) false false))

(event `self.Reachable.OnComponentBeginOverlap`
  (params (OverlappedComponent :type "PrimitiveComponent Object Reference") (OtherActor :type "Actor Object Reference") (OtherComp :type "PrimitiveComponent Object Reference") (OtherBodyIndex :type Integer) (bFromSweep :type Boolean) (SweepResult :type "HitResult Structure (by ref)"))
  ; Open On Player Reachable Area
  (`KismetSystemLibrary.IsObjectOfSoftClass` OtherActor "/Game/Blueprints/ThirdPersonPirate/BP_ThirdPersonCharacter.BP_ThirdPersonCharacter_C"
    (:`True`
      (if (not (`self.isChestOpen`))
        (`SkeletalMeshComponent.PlayAnimation` (`self.Mesh_ChestBase`) "/Game/Meshes/Chest/AS_OpenChest.AS_OpenChest" false)
        (set `self.isChestOpen` true)))))

(event `self.Reachable.OnComponentEndOverlap`
  (params (OverlappedComponent :type "PrimitiveComponent Object Reference") (OtherActor :type "Actor Object Reference") (OtherComp :type "PrimitiveComponent Object Reference") (OtherBodyIndex :type Integer))
  (bind _mesh_chestbase (`self.Mesh_ChestBase`))
  ; Close on player distance
  (`KismetSystemLibrary.IsObjectOfSoftClass` OtherActor "/Game/Blueprints/ThirdPersonPirate/BP_ThirdPersonCharacter.BP_ThirdPersonCharacter_C"
    (:`True`
      (if (not (not (`self.isChestOpen`)))
        (`SkeletalMeshComponent.PlayAnimation` _mesh_chestbase "/Game/Meshes/Chest/AS_CloseChest.AS_CloseChest" false)
        (`SkeletalMeshComponent.SetPosition` _mesh_chestbase 30.0 true)
        (set `self.isChestOpen` false)))))

(event `EvalShowTooltip_Event`
  (bind _backekey (`self.BackEKey`))
  (bind _frontekey (`self.FrontEkey`))
  ; Show/Hide Tooltip depend on children count
  (if (> (`KismetArrayLibrary.Array_Length` (`SceneComponent.GetChildrenComponents` (`self.DefaultSceneRoot`) false)) 4)
    (`SceneComponent.SetVisibility` _backekey true false)
    (`SceneComponent.SetVisibility` _frontekey true false)
    (else
      (`SceneComponent.SetVisibility` _backekey false false)
      (`SceneComponent.SetVisibility` _frontekey false false))))

(fn `UserConstructionScript`)