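; BP_PirateShip is a pirate ship actor that rocks gently to imitate floating on water.
; Tick adds a small local rotation from game-time sine waves, with separate frequencies for roll, pitch and yaw and a phase offset on yaw.
; The per-frame increments are not scaled by delta time, so the sway depends on frame rate.
; The construction script and other events are empty.
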(event `CustomEvent`)

(event `self.ReceiveTick`
  (params (DeltaSeconds :type "Float (single-precision)"))
  ; Water Effect rotation
  (`self.K2_AddActorLocalRotation` (`KismetMathLibrary.MakeRotator` (* (`KismetMathLibrary.Sin` (* (`KismetSystemLibrary.GetGameTimeInSeconds`) 0.75)) 0.004) (* (`KismetMathLibrary.Sin` (* (`KismetSystemLibrary.GetGameTimeInSeconds`) 0.6)) 0.004) (* (`KismetMathLibrary.Sin` (+ (* (`KismetSystemLibrary.GetGameTimeInSeconds`) 0.25) 1.5)) 0.002))))

(fn `UserConstructionScript`)