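; Pirate ship actor that gently rocks in place, as if riding waves.
; Each Tick sets an absolute actor rotation from sine waves of game time, with separate amplitudes for roll, pitch and yaw.
; Pitch swings faster than roll and yaw, and yaw is phase-shifted from roll.
; The computed rotation replaces any placed orientation, as the current rotation is not read.
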(event `CustomEvent`)

(event `self.ReceiveTick`
  (params (DeltaSeconds :type "Float (single-precision)"))
  (`self.K2_SetActorRotation` (`KismetMathLibrary.MakeRotator` (* (`KismetMathLibrary.Sin` (* (`KismetSystemLibrary.GetGameTimeInSeconds`) 0.2)) 1.5) (* (`KismetMathLibrary.Sin` (* (`KismetSystemLibrary.GetGameTimeInSeconds`) 0.5)) 2.0) (* (`KismetMathLibrary.Sin` (+ (* (`KismetSystemLibrary.GetGameTimeInSeconds`) 0.2) 1.5)) 0.5))))

(fn `UserConstructionScript`)